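; Fire Bolt gameplay ability that casts a projectile from the Aura player character toward the point under the mouse.
; On activation it commits, reads the cursor target data, turns the character to face that location and plays the cast montage.
; A montage gameplay event times the SpawnProjectile call to the animation.
; The ability ends when the montage completes, blends out, is interrupted or is cancelled.
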(event `self.K2_ActivateAbility`
  (`self.K2_CommitAbility`)
  (bind (_asynctaskproxy _data) (`TargetDataUnderMouse.CreateTargetDataUnderMouse`)
    (:`ValidData`
      (set `self.PrijectileTargetLocation` (`.Location` (`GameplayStatics.BreakHitResult` (`AbilitySystemBlueprintLibrary.GetHitResultFromTargetData` _data))))
      (bind _asbp_aura_character (cast `/Game/Blueprints/Character/Aura/BP_AuraCharacter` (`self.GetAvatarActorFromActorInfo`)))
      (bind _ascombat_interface (cast `CombatInterface` _asbp_aura_character))
      (`CombatInterface.UpdataFacingTarget` _ascombat_interface (`self.PrijectileTargetLocation`))
      (`AbilityTask_PlayMontageAndWait.CreatePlayMontageAndWaitProxy` "None" "/Game/Assets/Characters/Aura/Animations/Abilities/AM_Cast_FireBolt.AM_Cast_FireBolt" 1.0 "None" false
        (:`then`
          (`AbilityTask_WaitGameplayEvent.WaitGameplayEvent` (struct :`TagName` "Event.Montage.FireBolt") null
            (:`EventReceived`
              (`self.SpawnProjectile` (`self.PrijectileTargetLocation`)))))
        (:`OnCompleted`
          (`self.K2_EndAbility` :!label _label))
        (:`OnBlendOut`
          (goto _label))
        (:`OnInterrupted`
          (goto _label))
        (:`OnCancelled`
          (goto _label))))))